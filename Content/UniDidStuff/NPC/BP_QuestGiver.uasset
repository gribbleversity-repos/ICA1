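; BP_QuestGiver is a talkative NPC running a comedic branching dialogue that leads to revealing a keypad code.
; A passed-in widget supplies captions, portrait and two answer buttons, which a timeline reveals on interact.
; Each dialogue node is an event: Choice branches on the clicked button, then shows lines with random yap sounds and rebinds the YapThis dispatcher to the next node.
; Code endings hide the buttons and update BP_Rover's objective.
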(event `HereIsYourReferenceKing`
  (params (WidgetRef :type "/Game/UniDidStuff/Util/Widgets/W_RovingUI Object Reference"))
  (set `self.CaptionBox` (`/Game/UniDidStuff/Util/Widgets/W_RovingUI.Captions` WidgetRef))
  (set `self.Left` (`/Game/UniDidStuff/Util/Widgets/W_RovingUI.ButtonLeft` WidgetRef))
  (set `self.Right` (`/Game/UniDidStuff/Util/Widgets/W_RovingUI.ButtonRight` WidgetRef))
  (set `self.Left Shlarp` (`/Game/UniDidStuff/Util/Widgets/W_RovingUI.LeftShlarp` WidgetRef))
  (set `self.Right Shlarp` (`/Game/UniDidStuff/Util/Widgets/W_RovingUI.RightShlarp` WidgetRef))
  (set `self.LText` (`/Game/UniDidStuff/Util/Widgets/W_RovingUI.LText` WidgetRef))
  (set `self.RText` (`/Game/UniDidStuff/Util/Widgets/W_RovingUI.RText` WidgetRef))
  (set `self.Pfp` (`/Game/UniDidStuff/Util/Widgets/W_RovingUI.pfp` WidgetRef))
  (add `self.YapThis` (delegate `Start`))
  (`self.ButtonsSayWhaa` "hey little guy" "jeez ok im here"))

(event `Yap`
  (params (ClickedOnButton :type "Button Object Reference"))
  (set `self.Clicked on Button` ClickedOnButton)
  (`self.YapThis`))

(event `self.Sphere.OnComponentBeginOverlap`
  (params (OverlappedComponent :type "PrimitiveComponent Object Reference") (OtherActor :type "Actor Object Reference") (OtherComp :type "PrimitiveComponent Object Reference") (OtherBodyIndex :type Integer) (bFromSweep :type Boolean) (SweepResult :type "HitResult Structure (by ref)"))
  (`/Engine/EditorBlueprintResources/StandardMacros.DoOnce` false
    (:`Completed`
      (`self.SpeakYourTruthKing` "HEY YOU! YOU! YES YOU! COME HERE"))))

(event `self.Sphere.OnComponentEndOverlap`
  (params (OverlappedComponent :type "PrimitiveComponent Object Reference") (OtherActor :type "Actor Object Reference") (OtherComp :type "PrimitiveComponent Object Reference") (OtherBodyIndex :type Integer))
  (`self.SpeakYourTruthKing` ""))

(event `TheExit`
  (`self.Choice`
    (:`Left`
      (`self.Speak,GiveOptions,ConnectNext` "yes i am but thats irrelivent it wouldnt come up at all in this context at all. like yknow forgetting we ever had this conversation or anything like that" "chicken butt" "hey whats that over there?" (delegate `Dory`)))
    (:`Right`
      (`self.Speak,GiveOptions,ConnectNext` "Well.. its a bit akward.. you have to promise to not laugh ok?" "sure" "i make no promises" (delegate `Promise`) :!label _label))))

(event `LITTLE?`
  (`self.Choice`
    (:`Left`
      (`self.Speak,GiveOptions,ConnectNext` "thats the exit.. ive kinda been waiting for someone to open it for me.." "are you stupid?" "why would you need someone to open it for you?" (delegate `TheExit`) :!label _label_2))
    (:`Right`
      (`self.Speak,GiveOptions,ConnectNext` "right well i guess this is goodbye" "door. tell." "yap yap yap" (delegate `Goodbye?nuh`) :!label _label_3))))

(event `Dory`
  (`self.Speak,GiveOptions,ConnectNext` "w- where was i? oh yeah AUGHEUGH OUEAHGHOHG" "ARE YOU OK? WHAT IS GOING ON? HELLO? WHAT?" "get a grip." (delegate `WhereWasI`)))

(event `Start`
  (`self.Choice`
    (:`Left`
      (`self.Speak,GiveOptions,ConnectNext` "LITTLE? oh.. OH. so thats how it is.. i bet you dont even want to know about how to open this door anyway nono please go about your day its fine with me." "ok fine what is this door about?" "lit chill w/ me dawg" (delegate `LITTLE?`)))
    (:`Right`
      (`self.Speak,GiveOptions,ConnectNext` "ok ok sorry ive gotten a bit adgitated is all.. yknow since ive been stuck here for EIGHTY FOUR YEARS " "damn that sucks" "ok oldylocks" (delegate `84 years`) :!label _label_4))))

(event `RevealButtons`
  (bind (_direction _x _opacity) (`Timeline|swipe in from side` :!label _label_5)
    (:`Update`
      (`|ExecutionSequence`
        (:`then_0`
          (for _array_element (`|MakeArray` (`self.Left Shlarp`) (`self.Right Shlarp`) :!type "Widget Object Reference")
            (`self.SetXPosOfLeft&Right` _x _array_element)))
        (:`then_1`
          (set `Widget.RenderOpacity` _opacity (`self.Pfp`)))))))

(event `HideButtons`
  (goto _label_5 :!via `Reverse`))

(event `Goodbye?nuh`
  (`self.Choice`
    (:`Left`
      (goto _label_2))
    (:`Right`
      (`self.Speak,GiveOptions,ConnectNext` "oh. am i boring you? i bet you just want to know the code huh.. OR!! you could here my life story" "1 code to go please" "LIFE STORY" (delegate `LifeStory`) :!label _label_6))))

(event `84 years`
  (`self.Choice`
    (:`Left`
      (`self.Speak,GiveOptions,ConnectNext` "actually its not been that bad since ive just been on standby the whole time so once you got here it woke me up" "all i hear is yap" "wait so why have you been here so long" (delegate `Standby`)))
    (:`Right`
      (`self.Speak,GiveOptions,ConnectNext` "oldyWHAT... ok if anything if you think about it form factor wise, im smaller because the creators were able to compact things better MEANING im the upgrade MEANING im younger than you and ALSO outrank you" "me when i lie" "ok ok you outrank me, why have you been here so long" (delegate `oldyWHAT`)))))

(event `LifeStory`
  (`self.Choice`
    (:`Left`
      (`self.GiveCodeSpeedrunner`))
    (:`Right`
      (`self.Speak,GiveOptions,ConnectNext` "oh. i- i was bluffing.. 84 years of my life.. have been spent next to this door. its all i am. its all i do." "ok actually how have you done that" "surely you could have tried every combination by now" (delegate `Bluffing`)))))

(event `WhereWasI`
  (goto _label_4))

(event `Standby`
  (`self.Choice`
    (:`Left`
      (goto _label_6))
    (:`Right`
      (goto _label))))

(event `Bluffing`
  (`self.Choice`
    (:`Left`
      (goto _label))
    (:`Right`
      (`self.Speak,GiveOptions,ConnectNext` "ok.. so.. the.. well.. the keypad.. i.. i know the code.. theres just a.. well.. a uhm.. theres a height problem." "HAHAHAH HAHAUGHEAIOIUAG" "oh." (delegate `HeightProblem`) :!label _label_7))))

(event `ToldYou`
  (`self.Choice`
    (:`Left`
      (`self.Speak,GiveOptions,ConnectNext` "so uhm.. yeah.. if i tell you the code can you type it in for me..?" "yeah sure" "uhm.. do i get to leave too?" (delegate `TellingCode`) :!label _label_8))
    (:`Right`
      (`self.GiveCode (HesOfficiallyLostIt)`))))

(event `HeightProblem`
  (`self.Choice`
    (:`Left`
      (`self.Speak,GiveOptions,ConnectNext` "I TOLD YOU NOT TO LAUGH" "sorry sorry" "HUEAGH HOUGHEAOUGH HUEAH HUEAHEAHEAH" (delegate `ToldYou`)))
    (:`Right`
      (goto _label_8))))

(event `Promise`
  (`self.Choice`
    (:`Left`
      (goto _label_7))
    (:`Right`
      (`self.Speak,GiveOptions,ConnectNext` "YOU HAVE TO OK?" "why promise when i could just LEAVE" "i promise.." (delegate `SuperDuperPromise`)))))

(event `oldyWHAT`
  (`self.Choice`
    (:`Left`
      (`self.GiveCode (HesOfficiallyLostIt)`))
    (:`Right`
      (goto _label))))

(event `SuperDuperPromise`
  (`self.Choice`
    (:`Left`
      (goto _label_3))
    (:`Right`
      (goto _label_7))))

(event `TellingCode`
  (`self.Choice`
    (:`Left`
      (`self.GiveCodeApreaciate`))
    (:`Right`
      (`self.Speak,GiveOptions,ConnectNext` "well yeah if you are going to the exit that is" "awesome sauce" "exit? yes please" (delegate `yahyah`)))))

(event `GiveCode (HesOfficiallyLostIt)`
  (bind _returnvalue (`KismetStringLibrary.Conv_IntToString` (`/Game/UniDidStuff/Puzzles/KeyPad/BP_KeyPad.CorrectCode` (`self.KnownKeypad`))))
  (`self.Speak,GiveOptions,ConnectNext` (`KismetTextLibrary.Conv_StringToText` (`KismetStringLibrary.Concat_StrStr` "I WANT YOU TO LEAVE. THE CODE IS " _returnvalue " OK? WILL YOU PLEASE. PLEASE JUST LEAVE ME ALONE.")))
  (for _array_element (`|MakeArray` (`self.Left Shlarp`) (`self.Right Shlarp`)) :!label _label_9
    (set `Widget.Visibility` "Hidden" _array_element)
    (`/Game/UniDidStuff/Player/BP_Rover.UpdateObjective` (cast `/Game/UniDidStuff/Player/BP_Rover` (`GameplayStatics.GetPlayerPawn` 0) :!pure true) (`KismetStringLibrary.Concat_StrStr` "Enter code: " _returnvalue))))

(event `yahyah`
  (`self.GiveCodeApreaciate`))

(event `GiveCodeApreaciate`
  (`self.Speak,GiveOptions,ConnectNext` (`KismetTextLibrary.Conv_StringToText` (`KismetStringLibrary.Concat_StrStr` "the code for the keypad is " (`KismetStringLibrary.Conv_IntToString` (`/Game/UniDidStuff/Puzzles/KeyPad/BP_KeyPad.CorrectCode` (`self.KnownKeypad`))) " so if you would be so kind as to open the door with that it would be greatly apreaciated")))
  (goto _label_9))

(event `GiveCodeSpeedrunner`
  (`self.Speak,GiveOptions,ConnectNext` (`KismetTextLibrary.Conv_StringToText` (`KismetStringLibrary.Concat_StrStr` "silly little speedrunners ruining the deep lore ok fine its " (`KismetStringLibrary.Conv_IntToString` (`/Game/UniDidStuff/Puzzles/KeyPad/BP_KeyPad.CorrectCode` (`self.KnownKeypad`))) ", you're on pace for last in the world place btw")))
  (goto _label_9))

(fn `BindMyEvents`
  (params (Rover :type "/Game/UniDidStuff/Player/BP_Rover Object Reference"))
  (`parent.BindMyEvents` Rover)
  (`self.RevealButtons`))

(fn `ButtonsSayWhaa`
  (params (Left :type Text) (Right :type Text))
  (set `TextBlock.Text` Left (`self.LText`))
  (set `TextBlock.Text` Right (`self.RText`)))

(fn `IsLeft`
  (returns (ReturnValue :type Boolean))
  (return (== (`self.Clicked on Button`) (`self.Left`))))

(fn `SetXPosOfLeft&Right`
  (params (InPosition_X :type "Float (double-precision)") (WidgetComponent :type "Widget Object Reference"))
  (bind _returnvalue (`WidgetLayoutLibrary.SlotAsCanvasSlot` WidgetComponent))
  (bind (_returnvalue_x _returnvalue_y) (`KismetMathLibrary.BreakVector2D` (`CanvasPanelSlot.GetPosition` _returnvalue)))
  (`CanvasPanelSlot.SetPosition` _returnvalue (`KismetMathLibrary.MakeVector2D` (`KismetMathLibrary.SelectFloat` (/ InPosition_X -1.0) InPosition_X (== WidgetComponent (`self.Right Shlarp`))) _returnvalue_y)))

(fn `Speak & giveOptions`
  (params (Speak :type Text) (Left :type Text) (Right :type Text))
  (`self.SpeakYourTruthKing` Speak)
  (`self.ButtonsSayWhaa` Left Right))

(fn `Speak,GiveOptions,ConnectNext`
  (params (Speak :type Text) (Left :type Text) (Right :type Text) (NextYappingEvent :type Delegate))
  (`self.Speak & giveOptions` Speak Left Right)
  (`self.UnbindCurrentYapAndReadyNext` NextYappingEvent))

(fn `SpeakYourTruthKing`
  (params (KingsTruth :type Text))
  (set `TextBlock.Text` KingsTruth (`self.CaptionBox`))
  (`GameplayStatics.PlaySound2D` (select `int` (`KismetMathLibrary.RandomIntegerInRange` 0 5) :`0` "/Game/UniDidStuff/Audio/Yap0.Yap0" :`1` "/Game/UniDidStuff/Audio/Yap1.Yap1" :`2` "/Game/UniDidStuff/Audio/Yap2.Yap2" :`3` "/Game/UniDidStuff/Audio/Yap3.Yap3" :`4` "/Game/UniDidStuff/Audio/Yap4.Yap4" :`5` "/Game/UniDidStuff/Audio/Yap5.Yap5" :!type "SoundBase Object Reference") 1.0 1.0 0.0 null null))

(fn `UnbindCurrentYapAndReadyNext`
  (params (Event :type "Delegate (by ref)"))
  (clear `self.YapThis`)
  (add `self.YapThis` Event)
  (return))

(fn `Uninteract`
  (params (Rover :type "/Game/UniDidStuff/Player/BP_Rover Object Reference"))
  (`parent.Uninteract` Rover)
  (`self.HideButtons`))

(fn `UserConstructionScript`)