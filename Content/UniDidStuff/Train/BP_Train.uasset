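; BP_Train is a train actor whose body shuttles back and forth along the Y axis each time MoveMyJitty is called.
; A FlipFlop alternates between forward and backward arrows, line-tracing from the selected one to measure the distance to the first hit.
; Each call stops the opposite MoveComponentTo, then eases the body by that distance in positive or negative Y.
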(event `MoveMyJitty`
  (bind _body (`self.Body`))
  (bind (_returnvalue_x _returnvalue_y _returnvalue_z) (`KismetMathLibrary.BreakVector` (`SceneComponent.K2_GetComponentLocation` _body)))
  (bind _returnvalue (`SceneComponent.K2_GetComponentRotation` _body))
  (bind _output (`|GetArrayItem` (`|MakeArray` (`self.ArrowForward`) (`self.ArrowBackward`)) (`self.WhichArrow`)))
  (bind _returnvalue_2 (`SceneComponent.K2_GetComponentLocation` _output))
  (bind _isa (`/Engine/EditorBlueprintResources/StandardMacros.FlipFlop`)
    (:`A`
      (set `self.WhichArrow` 0))
    (:`B`
      (set `self.WhichArrow` 1)))
  (bind _outhit (`KismetSystemLibrary.LineTraceSingle` :`Start` _returnvalue_2 :`End` (+ _returnvalue_2 (* (`SceneComponent.GetForwardVector` _output) 5000)) :`TraceChannel` "TraceTypeQuery1" :`DrawDebugType` "ForDuration"))
  (if _isa
    (`|ExecutionSequence`
      (:`then_0`
        (goto _label_2 :!via `Stop`))
      (:`then_1`
        (bind (_bblockinghit _binitialoverlap _time _distance) (`GameplayStatics.BreakHitResult` _outhit))
        (`KismetSystemLibrary.MoveComponentTo` _body (`KismetMathLibrary.MakeVector` _returnvalue_x (+ _distance _returnvalue_y) _returnvalue_z) _returnvalue true true 2.5 :!label _label)))
    (else
      (`|ExecutionSequence`
        (:`then_0`
          (goto _label :!via `Stop`))
        (:`then_1`
          (`KismetSystemLibrary.MoveComponentTo` _body (`KismetMathLibrary.MakeVector` _returnvalue_x (- _returnvalue_y _distance) _returnvalue_z) _returnvalue true true 2.5 :!label _label_2))))))

(fn `UserConstructionScript`)