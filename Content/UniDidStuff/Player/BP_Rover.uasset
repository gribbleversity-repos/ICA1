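; Player character that walks, takes damage (death reloads the level), and operates interactable puzzle panels.
; Walk speed scales with movement direction relative to facing, and a HUD widget shows health and a toggleable, animated objective.
; Interacting sphere-traces for a BP_Interactable, then a FlipFlop timeline moves a secondary camera to or from it, swapping movement for mouse control.
; Rebindable press, release and camera-startup dispatchers route clicks to each panel type.
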(event `self.ReceiveBeginPlay`
  (`|ExecutionSequence`
    (:`then_0`
      ; add mapping context
      (bind _asplayer_controller (cast `PlayerController` (`self.GetController`)))
      (`EnhancedInputSubsystemInterface.AddMappingContext` (pcsubsystem `EnhancedInputLocalPlayerSubsystem` _asplayer_controller) "/Game/UniDidStuff/Player/Input/IMC_PlayerActions.IMC_PlayerActions" 0 (struct)))
    (:`then_1`
      (bind _returnvalue (`|CreateWidget` "/Game/UniDidStuff/Util/Widgets/W_RovingUI.W_RovingUI_C"))
      (`UserWidget.AddToViewport` _returnvalue 0)
      (bind _output_get (set `self.RovingUI` _returnvalue))
      (bind _outactors (`GameplayStatics.GetAllActorsOfClass` "/Game/UniDidStuff/NPC/BP_QuestGiver.BP_QuestGiver_C"))
      (for _array_element _outactors
        (`/Game/UniDidStuff/NPC/BP_QuestGiver.HereIsYourReferenceKing` _array_element _output_get)))
    (:`then_2`
      (`self.HideObjective`))))

(event `self.ReceiveAnyDamage`
  (params (Damage :type "Float (single-precision)") (DamageType :type "DamageType Object Reference") (InstigatedBy :type "Controller Object Reference") (DamageCauser :type "Actor Object Reference"))
  (bind _rovingui (`self.RovingUI`))
  (bind _output_get (set `self.Health` (- (`self.Health`) Damage)))
  (set `TextBlock.Text` (`KismetTextLibrary.Conv_StringToText` (`KismetStringLibrary.Concat_StrStr` "HP:   " (`KismetStringLibrary.Conv_DoubleToString` _output_get) "/100.0")) (`/Game/UniDidStuff/Util/Widgets/W_RovingUI.HealthText` _rovingui))
  (`ProgressBar.SetPercent` (`/Game/UniDidStuff/Util/Widgets/W_RovingUI.HealthBar` _rovingui) (/ _output_get 100.0))
  (if (<= _output_get 0.0)
    (`self.Die`)))

(event `Die`
  (bind _returnvalue (`GameplayStatics.GetCurrentLevelName` true))
  (`GameplayStatics.OpenLevel` (`KismetStringLibrary.Conv_StringToName` _returnvalue)))

(event `EnhancedInput|/Game/UniDidStuff/Player/Input/Actions/IA_SillyMove`
  (params (ActionValue :type "Vector2D Structure") (ElapsedSeconds :type "Float (double-precision)") (TriggeredSeconds :type "Float (double-precision)") (InputAction :type "InputAction Object Reference" :default "/Game/UniDidStuff/Player/Input/Actions/IA_SillyMove.IA_SillyMove"))
  (bind (_returnvalue_roll _returnvalue_pitch _returnvalue_yaw) (`KismetMathLibrary.BreakRotator` (`self.GetControlRotation`)))
  ;[0.76 0.1718 0 0.5] input
  ;; walk
  (:`Triggered`
    (`|ExecutionSequence`
      (:`then_0`
        (`self.CalculateNewWalkSpeed`))
      (:`then_1`
        (`self.AddMovementInput` (`KismetMathLibrary.GetRightVector` (`KismetMathLibrary.MakeRotator` _returnvalue_roll 0.0 _returnvalue_yaw)) ActionValue_X) ; Sideways
      )
      (:`then_2`
        (`self.AddMovementInput` (`KismetMathLibrary.GetForwardVector` (`KismetMathLibrary.MakeRotator` 0.0 0.0 _returnvalue_yaw)) ActionValue_Y) ; Frontfacing
      ))))

(event `CalculateNewWalkSpeed`
  ; Rover Turning Walk Speed
  (set `CharacterMovementComponent.MaxWalkSpeed` (* (* (- 1.0 (`KismetMathLibrary.MultiplyMultiply_FloatFloat` (- 1.0 (`KismetMathLibrary.FClamp` (/ (+ (`KismetMathLibrary.Dot_VectorVector` (`SceneComponent.GetForwardVector` (`self.CapsuleComponent`)) (`KismetMathLibrary.Normal` (`self.GetVelocity`))) 1.1) 2.0))) 4.0)) 600.0) (`self.SpeedModifier`)) (`self.CharacterMovement`)))

(event `UpdateObjective`
  (params (NewObjective :type String))
  (set `TextBlock.Text` (`KismetTextLibrary.Conv_StringToText` (`KismetStringLibrary.Concat_StrStr` "Current Objective: " NewObjective)) (`/Game/UniDidStuff/Util/Widgets/W_RovingUI.Objective` (`self.RovingUI`)))
  (`self.ShowObjective`))

(event `EnhancedInput|/Game/UniDidStuff/Player/Input/Actions/IA_ObjectiveToggle`
  (params (ActionValue :type Boolean) (ElapsedSeconds :type "Float (double-precision)") (TriggeredSeconds :type "Float (double-precision)") (InputAction :type "InputAction Object Reference" :default "/Game/UniDidStuff/Player/Input/Actions/IA_ObjectiveToggle.IA_ObjectiveToggle"))
  ;[0.76 0.1718 0 0.5] input
  ;; show/hide objective
  (:`Started`
    (switch `ETimelineDirection` (stale `ShowObjective` _direction)
      (:`Forward`
        (`self.HideObjective`))
      (:`Backward`
        (`self.ShowObjective`)))))

(event `ShowObjective`
  (bind (_direction _x _y) (`Timeline|show me that objective oh yeah` :!label _label)
    (:`Update`
      (`CanvasPanelSlot.SetPosition` (`WidgetLayoutLibrary.SlotAsCanvasSlot` (`/Game/UniDidStuff/Util/Widgets/W_RovingUI.Objective` (`self.RovingUI`))) (`KismetMathLibrary.MakeVector2D` _x _y)))
    (:`PlaySound`
      (`GameplayStatics.PlaySound2D` (select `ETimelineDirection` _direction :`Forward` "/Game/UniDidStuff/Audio/ObjectiveOn.ObjectiveOn" :`Backward` "/Game/UniDidStuff/Audio/ObjectiveOff.ObjectiveOff" :!type "SoundBase Object Reference") 1.0 1.0 0.0 null null))))

(event `HideObjective`
  (goto _label :!via `Reverse`))

(event `EnhancedInput|/Game/UniDidStuff/Player/Input/Actions/IA_SillyLook`
  (params (ActionValue :type "Vector2D Structure") (ElapsedSeconds :type "Float (double-precision)") (TriggeredSeconds :type "Float (double-precision)") (InputAction :type "InputAction Object Reference" :default "/Game/UniDidStuff/Player/Input/Actions/IA_SillyLook.IA_SillyLook"))
  ;[0.76 0.1718 0 0.5] input
  ;; camera movement
  (:`Triggered`
    (`/Engine/EditorBlueprintResources/StandardMacros.Gate` false :!label _label_2
      (:`Exit`
        (`|ExecutionSequence`
          (:`then_0`
            (`self.AddControllerYawInput` ActionValue_X))
          (:`then_1`
            (`self.AddControllerPitchInput` ActionValue_Y)))))))

(event `EnhancedInput|/Game/UniDidStuff/Player/Input/Actions/IA_SillyPannelClick`
  (params (ActionValue :type Boolean) (ElapsedSeconds :type "Float (double-precision)") (TriggeredSeconds :type "Float (double-precision)") (InputAction :type "InputAction Object Reference" :default "/Game/UniDidStuff/Player/Input/Actions/IA_SillyPannelClick.IA_SillyPannelClick"))
  ;[0.76 0.1718 0 0.5] input
  ;; pannelclick
  (:`Started`
    (`self.PannelPress`))
  (:`Completed`
    (`self.PannelRelease`)))

(event `EnableCamMovement`
  ;[0.76 0.1718 0 0.5] input
  ;; camera movement
  (goto _label_2 :!via `Open`))

(event `DisableCamMovement`
  ;[0.76 0.1718 0 0.5] input
  ;; camera movement
  (goto _label_2 :!via `Close`))

(event `KickOut`
  (params (PanelExiting :type "Actor Object Reference"))
  ;[0.76 0.1718 0 0.5] input
  ;; interact
  (set `self.KickingOut?` true)
  (bind (_bblockinghit _binitialoverlap _time _distance _location _impactpoint _normal _impactnormal _physmat _hitactor) (`GameplayStatics.BreakHitResult` (stale `EnhancedInput|/Game/UniDidStuff/Player/Input/Actions/IA_SillyInteract` _outhit)))
  (bind _asbp_interactable (cast `/Game/UniDidStuff/Util/BP_Interactable` (`KismetMathLibrary.SelectObject` PanelExiting _hitactor (`self.KickingOut?`)) :!label _label_3))
  (`/Engine/EditorBlueprintResources/StandardMacros.IsValid` (`self.CurrentPannel`)
    (:`Is Valid`
      (`/Game/UniDidStuff/Util/BP_Interactable.Uninteract` _asbp_interactable self)
      (set `self.CurrentPannel` null))
    (:`Is Not Valid`
      (set `self.CurrentPannel` _hitactor)
      (`/Game/UniDidStuff/Util/BP_Interactable.BindMyEvents` _asbp_interactable self)))
  (bind _cameratarget (`/Game/UniDidStuff/Util/BP_Interactable.CameraTarget` _asbp_interactable))
  (`self.2ndCamMoveToPosAndEnableToggler` (`SceneComponent.K2_GetComponentRotation` _cameratarget) (`SceneComponent.K2_GetComponentLocation` _cameratarget)))

(event `EnhancedInput|/Game/UniDidStuff/Player/Input/Actions/IA_SillyInteract`
  (params (ActionValue :type Boolean) (ElapsedSeconds :type "Float (double-precision)") (TriggeredSeconds :type "Float (double-precision)") (InputAction :type "InputAction Object Reference" :default "/Game/UniDidStuff/Player/Input/Actions/IA_SillyInteract.IA_SillyInteract"))
  (bind _returnvalue (+ (`SceneComponent.K2_GetComponentLocation` (`self.CapsuleComponent`)) (0.0 0.0 100.0)))
  ;[0.76 0.1718 0 0.5] input
  ;; interact
  (:`Started`
    (bind _outhit (`KismetSystemLibrary.SphereTraceSingleForObjects` :`Start` _returnvalue :`End` (+ _returnvalue (* (`KismetMathLibrary.GetForwardVector` (`self.GetControlRotation`)) 200)) :`Radius` 60.0 :`ObjectTypes` (`|MakeArray` "ObjectTypeQuery1" :!type "EObjectTypeQuery Enum") :`DrawTime` 0.2))
    (bind (_bblockinghit _binitialoverlap _time _distance _location _impactpoint _normal _impactnormal _physmat _hitactor) (`GameplayStatics.BreakHitResult` _outhit))
    (if _bblockinghit
      (if (`KismetMathLibrary.ClassIsChildOf` (`GameplayStatics.GetObjectClass` _hitactor) "/Game/UniDidStuff/Util/BP_Interactable.BP_Interactable_C")
        (set `self.KickingOut?` false)
        (goto _label_3)))))

(event `2ndCamMoveToPosAndEnableToggler`
  (params (EndGoalRot :type "Rotator Structure") (EndGoalPos :type "Vector Structure"))
  (bind _returnvalue (`GameplayStatics.GetPlayerController` 0))
  (bind _returnvalue_2 (`GameplayStatics.GetPlayerController` 0))
  (bind _charactermovement (`self.CharacterMovement`))
  (bind _hoveringcamera (`self.HoveringCamera`))
  (bind _hoveringcamera_2 (`self.HoveringCamera`))
  (bind (_x _y) (`KismetMathLibrary.BreakVector2D` (/ (`WidgetLayoutLibrary.GetViewportSize`) 2.0)))
  (`|ExecutionSequence`
    (:`then_0`
      ; if we dont do this then if we return we snap to the middle first of all
      (bind _returnvalue_3 (`SceneComponent.K2_GetComponentRotation` (`self.SecondaryCamera`))))
    (:`then_1`
      (`|ExecutionSequence`
        (:`then_0`
          (bind _returnvalue_4 (`SceneComponent.K2_GetComponentRotation` _hoveringcamera)))
        (:`then_1`
          (bind _returnvalue_5 (`SceneComponent.K2_GetComponentLocation` _hoveringcamera)))
        (:`then_2`
          (bind _isa (`/Engine/EditorBlueprintResources/StandardMacros.FlipFlop`) ; A = Going to point\nB = Coming back to player
            (:`A`
              (`self.DisableCamMovement`)
              (`ActorComponent.SetActive` _hoveringcamera_2 false false)
              (`CharacterMovementComponent.SetMovementMode` _charactermovement "MOVE_None" 0)
              (set `self.2ndCamMoving` true)
              (bind (_direction _lerp_alpha) (`Timeline|Timeline` :!label _label_4)
                (:`Update`
                  (`SceneComponent.K2_SetWorldLocationAndRotation` (`self.SecondaryCamera`) (`KismetMathLibrary.VLerp` _returnvalue_5 EndGoalPos _lerp_alpha) (`KismetMathLibrary.RLerp` _returnvalue_4 (`KismetMathLibrary.SelectRotator` EndGoalRot _returnvalue_3 (and _isa (`self.2ndCamMoving`))) _lerp_alpha true) false true))
                (:`Finished`
                  (set `self.2ndCamMoving` false)
                  (if _isa
                    (`PlayerController.SetMouseLocation` _returnvalue_2 (`KismetMathLibrary.FTrunc` _x) (`KismetMathLibrary.FTrunc` _y))
                    ; Control mouse
                    (set `PlayerController.bShowMouseCursor` true _returnvalue_2)
                    (`WidgetBlueprintLibrary.SetInputMode_GameAndUIEx` _returnvalue_2 null "DoNotLock" false)
                    (`self.PannelStartupCameraRotation`)
                    (set `self.SillyBaseRotation` (`SceneComponent.RelativeRotation` (`self.SecondaryCamera`)))
                    (else
                      (`CharacterMovementComponent.SetMovementMode` _charactermovement "MOVE_Walking" 0)
                      (`ActorComponent.SetActive` _hoveringcamera_2 true false)
                      ; Control camera
                      (set `PlayerController.bShowMouseCursor` false _returnvalue)
                      (`WidgetBlueprintLibrary.SetInputMode_GameOnly` _returnvalue)
                      (`self.EnableCamMovement`))))))
            (:`B`
              (`self.StopCameraRoationUpdating`)
              (`self.UnbindAllPanelEvents`)
              (goto _label_4 :!via `Reverse`))))))))

(event `BindTicketMachinePanelStuff`
  ; ticket machine events
  (add `self.PannelPress` (delegate `PanP_TicketMachine`)))

(event `PanP_TicketMachine`
  ; ticket machine events
  (bind _asbp_ticket_machine (cast `/Game/UniDidStuff/TicketMachine/BP_TicketMachine` (`self.CurrentPannel`)))
  (`/Game/UniDidStuff/TicketMachine/BP_TicketMachine.AttemptButtonPress` _asbp_ticket_machine))

(event `BindKeyPadPanelStuff`
  ; keybad events
  (add `self.PannelPress` (delegate `PanP_KeyPad`)))

(event `BindFlipperPannelStuff`
  ; flipper events
  (add `self.PannelPress` (delegate `PanP_Flipper`)))

(event `PanP_KeyPad`
  ; keybad events
  (bind _asbp_key_pad (cast `/Game/UniDidStuff/Puzzles/KeyPad/BP_KeyPad` (`self.CurrentPannel`)))
  (`/Game/UniDidStuff/Puzzles/KeyPad/BP_KeyPad.ClickOnButtonsTrace` _asbp_key_pad))

(event `PanP_Flipper`
  ; flipper events
  (bind _asbp_flipper (cast `/Game/UniDidStuff/Puzzles/Flipper/BP_Flipper` (`self.CurrentPannel`)))
  (`/Game/UniDidStuff/Puzzles/Flipper/BP_Flipper.try to flick switch` _asbp_flipper))

(event `BindWireBoxPanelStuff`
  ; wirebox events
  (add `self.PannelPress` (delegate `PanP_WireBox`))
  (add `self.PannelRelease` (delegate `PanR_WireBox`))
  (add `self.PannelStartupCameraRotation` (delegate `PanSCR_Play`)))

(event `PanP_WireBox`
  ; wirebox events
  (bind _asbp_wire_box (cast `/Game/UniDidStuff/Puzzles/Wires/BP_WireBox` (`self.CurrentPannel`)))
  (`/Game/UniDidStuff/Puzzles/Wires/BP_WireBox.AttemptWireGrab` _asbp_wire_box))

(event `PanR_WireBox`
  ; wirebox events
  (bind _asbp_wire_box (cast `/Game/UniDidStuff/Puzzles/Wires/BP_WireBox` (`self.CurrentPannel`)))
  (`/Game/UniDidStuff/Puzzles/Wires/BP_WireBox.ReleaseWire` _asbp_wire_box))

(event `PanSCR_Play`
  (bind (_returnvalue_x _returnvalue_y) (`KismetMathLibrary.BreakVector2D` (`WidgetLayoutLibrary.GetViewportSize`)))
  (bind (_sillybaserotation_roll _sillybaserotation_pitch _sillybaserotation_yaw) (`KismetMathLibrary.BreakRotator` (`self.SillyBaseRotation`)))
  (bind (_locationx _locationy) (`PlayerController.GetMousePosition` (`GameplayStatics.GetPlayerController` 0)))
  (bind _returnvalue (/ _locationx _returnvalue_x))
  (bind _returnvalue_2 (/ _locationy _returnvalue_y))
  (`Timeline|Timeline_0` :!label _label_5
    (:`Update`
      (`KismetSystemLibrary.PrintString` (`KismetStringLibrary.Concat_StrStr` "Mouse Pos - " "X: " (`KismetStringLibrary.Conv_DoubleToString` _locationx) " // " "Y; " (`KismetStringLibrary.Conv_DoubleToString` _locationy)) true false (struct :`R` 0.090137 :`G` 0.47 :`A` 1.0) 2.0 "h798ruhn")
      (`KismetSystemLibrary.PrintString` (`KismetStringLibrary.Concat_StrStr` "Viewport Size - " "X: " (`KismetStringLibrary.Conv_DoubleToString` _returnvalue_x) " // " "Y: " (`KismetStringLibrary.Conv_DoubleToString` _returnvalue_y)) true false (struct :`G` 0.012671 :`B` 0.37 :`A` 1.0) 2.0 "n430ruy")
      (`KismetSystemLibrary.PrintString` (`KismetStringLibrary.Concat_StrStr` "Distance across screen - " "X: " (`KismetStringLibrary.Conv_DoubleToString` _returnvalue) " // " "Y: " (`KismetStringLibrary.Conv_DoubleToString` _returnvalue_2)) true false (struct :`R` 1.0 :`G` 0.02 :`B` 0.02 :`A` 1.0) 2.0 "djjyfdgs")
      (`SceneComponent.K2_SetRelativeRotation` (`self.SecondaryCamera`) (`KismetMathLibrary.MakeRotator` 180.0 (+ (+ _sillybaserotation_pitch (* (`KismetMathLibrary.Lerp` _returnvalue_2 0.5 0.85) 360.0)) 0.5) (+ (+ (* (`KismetMathLibrary.Lerp` _returnvalue 0.5 0.85) 360.0) _sillybaserotation_yaw) 0.5)) false false))))

(event `StopCameraRoationUpdating`
  (goto _label_5 :!via `Stop`))

(fn `UnbindAllPanelEvents`
  (clear `self.PannelPress`)
  (clear `self.PannelRelease`)
  (clear `self.PannelStartupCameraRotation`))

(fn `UserConstructionScript`)