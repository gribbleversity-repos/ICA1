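; BP_Globe is an interactive globe that animates and displays its yaw while the third-person character is inside its sphere trigger.
; Entering plays timelines that scale it, bob it around its BeginPlay height, spin it a fixed step per update, and turn the text toward the follow camera.
; A delayed loop refreshes the yaw text every second.
; Leaving stops rotation, reverses scaling and hides the text, but the loop keeps running.
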(event `self.Sphere.OnComponentBeginOverlap`
  (params (OverlappedComponent :type "PrimitiveComponent Object Reference") (OtherActor :type "Actor Object Reference") (OtherComp :type "PrimitiveComponent Object Reference") (OtherBodyIndex :type Integer) (bFromSweep :type Boolean) (SweepResult :type "HitResult Structure (by ref)"))
  (bind _globe (`self.globe`))
  (bind _textrender (`self.TextRender`))
  (bind (_returnvalue_x _returnvalue_y) (`KismetMathLibrary.BreakVector` (`SceneComponent.K2_GetComponentLocation` _globe)))
  (bind (_returnvalue_roll _returnvalue_pitch _returnvalue_yaw) (`KismetMathLibrary.BreakRotator` (`SceneComponent.K2_GetComponentRotation` (`self.globe`))))
  ; this isnt 90 degrees each second // change it
  (cast `/Game/ThirdPerson/Blueprints/BP_ThirdPersonCharacter` OtherActor)
  (`|ExecutionSequence`
    (:`then_0`
      (bind (_direction _bobbing) (`Timeline|RotateBrah` :!label _label)
        (:`Update`
          (bind _output_get (set `self.RotatyBlahBlah` (+ (`self.RotatyBlahBlah`) 1.5)))
          (`SceneComponent.K2_SetRelativeRotation` _globe (`KismetMathLibrary.MakeRotator` 0.0 0.0 _output_get) false false)
          (`SceneComponent.K2_SetWorldLocation` _globe (`KismetMathLibrary.MakeVector` _returnvalue_x _returnvalue_y (+ _bobbing (.z (stale `self.ReceiveBeginPlay` _returnvalue)))) false false)
          (bind _asbp_third_person_character (cast `/Game/ThirdPerson/Blueprints/BP_ThirdPersonCharacter` (`GameplayStatics.GetPlayerPawn` 0)))
          (`SceneComponent.K2_SetRelativeRotation` _textrender (`KismetMathLibrary.FindLookAtRotation` (`SceneComponent.K2_GetComponentLocation` _textrender) (`SceneComponent.K2_GetComponentLocation` (`/Game/ThirdPerson/Blueprints/BP_ThirdPersonCharacter.FollowCamera` _asbp_third_person_character))) false false))))
    (:`then_1`
      (bind (_direction_2 _heyyy) (`Timeline|Scale` :!label _label_2)
        (:`Update`
          (`SceneComponent.SetRelativeScale3D` (`self.globe`) (`KismetMathLibrary.Conv_DoubleToVector` _heyyy)))))
    (:`then_2`
      (`KismetSystemLibrary.Delay` 1.0)
      (`SceneComponent.SetVisibility` (`self.TextRender`) true false)
      (`TextRenderComponent.K2_SetText` (`self.TextRender`) (`KismetTextLibrary.Conv_DoubleToText` _returnvalue_yaw "HalfToEven") :!label _label_3)
      (`KismetSystemLibrary.Delay` 1.0)
      (goto _label_3))))

(event `self.Sphere.OnComponentEndOverlap`
  (params (OverlappedComponent :type "PrimitiveComponent Object Reference") (OtherActor :type "Actor Object Reference") (OtherComp :type "PrimitiveComponent Object Reference") (OtherBodyIndex :type Integer))
  ; this isnt 90 degrees each second // change it
  (cast `/Game/ThirdPerson/Blueprints/BP_ThirdPersonCharacter` OtherActor)
  (`|ExecutionSequence`
    (:`then_0`
      (goto _label :!via `Stop`))
    (:`then_1`
      (goto _label_2 :!via `Reverse`))
    (:`then_2`
      (`KismetSystemLibrary.Delay` 0.3)
      (`SceneComponent.SetVisibility` (`self.TextRender`) false false))))

(event `self.ReceiveBeginPlay`
  ; this isnt 90 degrees each second // change it
  (bind _returnvalue (`SceneComponent.K2_GetComponentLocation` (`self.globe`))))

(fn `UserConstructionScript`)