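; Ticket machine actor that dispenses a single ticket when its button is clicked and lets the player take it.
; AttemptButtonPress sphere-traces from the mouse cursor to detect the Button or Ticket component.
; The button animates in and back behind a resetting DoOnce, while a second DoOnce limits ticket ejection to once.
; A taken ticket flies toward CameraTarget before being destroyed; BindMyEvents delegates panel binding to the Rover.
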(event `AttemptButtonPress`
  (bind _button (`self.Button`))
  (bind (_worldlocation _worlddirection) (`PlayerController.DeprojectMousePositionToWorld` (`GameplayStatics.GetPlayerController` 0)))
  (bind _relativerotation (`SceneComponent.RelativeRotation` _button))
  (bind (_outhit _returnvalue) (`KismetSystemLibrary.SphereTraceSingleForObjects` :`Start` _worldlocation :`End` (+ _worldlocation (* _worlddirection 500)) :`Radius` 5.0 :`ObjectTypes` (`|MakeArray` "ObjectTypeQuery2" :!type "EObjectTypeQuery Enum") :`DrawDebugType` "ForDuration" :`bIgnoreSelf` false :`DrawTime` 0.2))
  (if _returnvalue
    (bind (_bblockinghit _binitialoverlap _time _distance _location _impactpoint _normal _impactnormal _physmat _hitactor _hitcomponent) (`GameplayStatics.BreakHitResult` _outhit))
    (if (== _hitcomponent _button)
      (`/Engine/EditorBlueprintResources/StandardMacros.DoOnce` false :!label _label
        (:`Completed`
          (set `self.ReturnPos` (`SceneComponent.RelativeLocation` _button))
          (`KismetSystemLibrary.MoveComponentTo` _button (+ (`self.ReturnPos`) (-80.0 0.0 0.0)) _relativerotation true true)
          (`KismetSystemLibrary.MoveComponentTo` _button (`self.ReturnPos`) _relativerotation true true)
          (`|ExecutionSequence`
            (:`then_0`
              (`/Engine/EditorBlueprintResources/StandardMacros.DoOnce` false
                (:`Completed`
                  (`self.OutComesTheTicket`))))
            (:`then_1`
              (goto _label :!via `Reset`)))))
      (elif (== _hitcomponent (`self.Ticket`))
        (`self.TakeTicket`)))))

(event `OutComesTheTicket`
  (bind _ticket (`self.Ticket`))
  (`KismetSystemLibrary.MoveComponentTo` _ticket (+ (`SceneComponent.RelativeLocation` _ticket) (225.0 0.0 0.0)) (`SceneComponent.RelativeRotation` _ticket) true))

(event `TakeTicket`
  (bind _ticket (`self.Ticket`))
  (bind _cameratarget (`self.CameraTarget`))
  (bind (_relativerotation_roll _relativerotation_pitch _relativerotation_yaw) (`KismetMathLibrary.BreakRotator` (`SceneComponent.RelativeRotation` _cameratarget)))
  (`KismetSystemLibrary.MoveComponentTo` _ticket (+ (`SceneComponent.RelativeLocation` _cameratarget) (700.0 0.0 -100.0)) (`KismetMathLibrary.MakeRotator` _relativerotation_roll (+ _relativerotation_pitch 90.0) _relativerotation_yaw) true true 0.4)
  (`ActorComponent.K2_DestroyComponent` _ticket))

(fn `BindMyEvents`
  (params (Rover :type "/Game/UniDidStuff/Player/BP_Rover Object Reference"))
  (`/Game/UniDidStuff/Player/BP_Rover.BindTicketMachinePanelStuff` Rover))

(fn `UserConstructionScript`)