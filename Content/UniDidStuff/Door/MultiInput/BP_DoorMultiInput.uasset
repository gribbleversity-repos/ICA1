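; BP_DoorMultiInput is a door that opens once its accumulated power reaches a required threshold and closes when it drops below.
; UpdatePower adds each incoming difference to Power, refreshes the lights, then triggers Open or Close.
; The child components of Lights act as a progress display, turning green up to the Power count and red beyond.
; MoveComponentTo slides Cover sideways from the closed position cached by the construction script.
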(event `Open`
  (bind _cover (`self.Cover`))
  (`KismetSystemLibrary.MoveComponentTo` _cover (- (`self.ClosedPos`) (0.0 300.0 0.0)) (`SceneComponent.RelativeRotation` _cover) true false 2.0))

(event `UpdatePower`
  (params (PowerDifference :type Integer))
  (bind _output_get (set `self.Power` (+ PowerDifference (`self.Power`))))
  (`self.UpdateLights`)
  (if (>= _output_get (`self.RequiredPower`))
    (`self.Open`)
    (else
      (`self.Close`))))

(event `Close`
  (bind _cover (`self.Cover`))
  (`KismetSystemLibrary.MoveComponentTo` _cover (`self.ClosedPos`) (`SceneComponent.RelativeRotation` _cover) true false 2.0))

(event `UpdateLights`
  (for (_array_element _array_index) (`SceneComponent.GetChildrenComponents` (`self.Lights`) false)
    (bind _asprimitive_component (cast `PrimitiveComponent` _array_element))
    (`PrimitiveComponent.SetMaterial` _asprimitive_component 0 (select `bool` (<= (+ _array_index 1) (`self.Power`)) :`false` "/Game/UniDidStuff/Door/MultiInput/Materials/MAT_Light_Red.MAT_Light_Red" :`true` "/Game/UniDidStuff/Door/MultiInput/Materials/MAT_Light_Green.MAT_Light_Green" :!type "MaterialInterface Object Reference"))))

(fn `UserConstructionScript`
  (set `self.ClosedPos` (`SceneComponent.RelativeLocation` (`self.Cover`))))