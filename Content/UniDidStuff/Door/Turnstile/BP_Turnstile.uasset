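; Turnstile door that lets the player's Rover push through once AllowEntry turns its invisible wall into a trigger.
; AllowEntry opens two gates that pass the trigger's begin and end overlaps, starting and stopping the timelines.
; A SetNewTime timeline continually scrubs the Rotate timeline by player position along the axis chosen from Connecter's orientation.
; Rotate pitches the Twister and sets the Rover's speed modifier, which resets to normal on exit.
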(event `AllowEntry`
  (bind (_returnvalue_x _returnvalue_y) (`KismetMathLibrary.BreakVector` (`SceneComponent.K2_GetComponentLocation` (`self.Twister`))))
  (bind _returnvalue_x_2 (`KismetMathLibrary.BreakVector` (`SceneComponent.GetRightVector` (`self.Connecter`))))
  (bind _returnvalue (== _returnvalue_x_2 1.0))
  (`PrimitiveComponent.SetCollisionProfileName` (`self.Invisible(Wall / Trigger)`) "Trigger" true)
  (`KismetSystemLibrary.DelayUntilNextTick`)
  (`|ExecutionSequence`
    (:`then_0`
      (goto _label :!via `Open`))
    (:`then_1`
      (goto _label_4 :!via `Open`))))

(event `self.Invisible(Wall / Trigger).OnComponentBeginOverlap`
  (params (OverlappedComponent :type "PrimitiveComponent Object Reference") (OtherActor :type "Actor Object Reference") (OtherComp :type "PrimitiveComponent Object Reference") (OtherBodyIndex :type Integer) (bFromSweep :type Boolean) (SweepResult :type "HitResult Structure (by ref)"))
  (bind (_returnvalue_x _returnvalue_y) (`KismetMathLibrary.BreakVector` (`self.K2_GetActorLocation` OtherActor)))
  (bind (_returnvalue_x_2 _returnvalue_y_2) (`KismetMathLibrary.BreakVector` (`SceneComponent.K2_GetComponentLocation` (`self.Twister`))))
  (bind _returnvalue_x_3 (`KismetMathLibrary.BreakVector` (`SceneComponent.GetRightVector` (`self.Connecter`))))
  (bind _returnvalue (== _returnvalue_x_3 1.0))
  (`/Engine/EditorBlueprintResources/StandardMacros.Gate` true :!label _label
    (:`Exit`
      (if (== (`GameplayStatics.GetPlayerPawn` 0) OtherActor)
        (`|ExecutionSequence`
          (:`then_0`
            (bind _asbp_rover (cast `/Game/UniDidStuff/Player/BP_Rover` (`GameplayStatics.GetPlayerPawn` 0))))
          (:`then_1`
            (`Timeline|SetNewTime` :!label _label_2
              (:`Update`
                (bind (_direction _y _roverspeedmodifier) (`Timeline|Rotate` :`NewTime` (/ (+ (- (select `bool` _returnvalue :`false` _returnvalue_x :`true` _returnvalue_y) (select `bool` _returnvalue :`false` _returnvalue_x_2 :`true` _returnvalue_y_2)) 145.0) 290.0) :!via `SetNewTime` :!label _label_3)
                  (:`Update`
                    (`SceneComponent.K2_SetRelativeRotation` (`self.Twister`) (`KismetMathLibrary.MakeRotator` 0.0 (`KismetMathLibrary.SelectFloat` (/ _y -1.0) _y _returnvalue)) false false)
                    (set `/Game/UniDidStuff/Player/BP_Rover.SpeedModifier` _roverspeedmodifier _asbp_rover))))))
          (:`then_2`
            (goto _label_3)))))))

(event `self.Invisible(Wall / Trigger).OnComponentEndOverlap`
  (params (OverlappedComponent :type "PrimitiveComponent Object Reference") (OtherActor :type "Actor Object Reference") (OtherComp :type "PrimitiveComponent Object Reference") (OtherBodyIndex :type Integer))
  (`/Engine/EditorBlueprintResources/StandardMacros.Gate` true :!label _label_4
    (:`Exit`
      (`KismetSystemLibrary.PrintString` "bye")
      (if (== (`GameplayStatics.GetPlayerPawn` 0) OtherActor)
        (`|ExecutionSequence`
          (:`then_0`
            (goto _label_3 :!via `Stop`))
          (:`then_1`
            (goto _label_2 :!via `Stop`))
          (:`then_2`
            (set `/Game/UniDidStuff/Player/BP_Rover.SpeedModifier` 1.0 (stale `self.Invisible(Wall / Trigger).OnComponentBeginOverlap` _asbp_rover))))))))

(fn `UserConstructionScript`)