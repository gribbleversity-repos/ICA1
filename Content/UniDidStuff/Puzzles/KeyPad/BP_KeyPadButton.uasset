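; BP_KeyPadButton is a keypad puzzle button that animates a press when its PushButton event is called.
; The construction script stores the Button component's resting relative location.
; PushButton swaps the material to M_TaskExit and uses MoveComponentTo to slide the button a short way along negative X.
; It then moves the button back to rest and sets the material to M_SimpleFlatColour.
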(event `PushButton`
  (bind _button (`self.Button`))
  (`PrimitiveComponent.SetMaterial` _button 0 "/Game/Scenarios/BaseContent/Materials/Bases/M_TaskExit.M_TaskExit")
  (`KismetSystemLibrary.MoveComponentTo` _button (+ (`self.ReturnPos`) (-5.0 0.0 0.0)) (`SceneComponent.RelativeRotation` _button) :!label _label)
  (`KismetSystemLibrary.MoveComponentTo` _button (`self.ReturnPos`) (`SceneComponent.RelativeRotation` _button))
  (`|ExecutionSequence`
    (:`then_0`
      (goto _label :!via `Return`))
    (:`then_1`
      (`PrimitiveComponent.SetMaterial` _button 0 "/Game/Scenarios/BaseContent/Materials/Bases/M_SimpleFlatColour.M_SimpleFlatColour"))))

(event `aaaa`)

(fn `UserConstructionScript`
  (set `self.ReturnPos` (`SceneComponent.RelativeLocation` (`self.Button`))))