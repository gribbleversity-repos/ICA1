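; A keypad puzzle panel that opens a linked door when the player enters a randomly generated four-digit code.
; On BeginPlay it picks the code and writes it to a connected clue.
; A sphere trace from the mouse cursor presses keypad buttons, while number, backspace and enter events edit and check the screen text.
; Errors flash the text red; success flashes green, kicks out the Rover pawn and moves the door.
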(event `ClickOnButtonsTrace`
  (bind (_worldlocation _worlddirection) (`PlayerController.DeprojectMousePositionToWorld` (`GameplayStatics.GetPlayerController` 0)))
  (bind _outhit (`KismetSystemLibrary.SphereTraceSingleForObjects` _worldlocation (+ _worldlocation (* _worlddirection 500)) 5.0 (`|MakeArray` "ObjectTypeQuery2" :!type "EObjectTypeQuery Enum") false (`self.IgnoreInTrace`) "None" false (struct :`R` 1.0 :`A` 1.0) (struct :`G` 1.0 :`A` 1.0) 0.2))
  (bind _asbp_key_pad_button (cast `/Game/UniDidStuff/Puzzles/KeyPad/BP_KeyPadButton` (`.HitActor` (`GameplayStatics.BreakHitResult` _outhit))))
  (`/Game/UniDidStuff/Puzzles/KeyPad/BP_KeyPadButton.PushButton` _asbp_key_pad_button))

(event `PushNumber`
  (params (ButtonNumber :type Integer))
  (bind _addednumber (`self.AddNumberToScreen` 6 ButtonNumber))
  (if (not _addednumber)
    (`self.SetColourThenWhite` 0 0 255)))

(event `PushBackspace`
  (`self.RemoveLastDigit`))

(event `PushEnter`
  (if (`KismetTextLibrary.EqualEqual_TextText` (`TextRenderComponent.Text` (`self.ScreenText`)) (`|FormatText` (`KismetTextLibrary.Conv_IntToText` (`self.CorrectCode`) false false)))
    (`|ExecutionSequence`
      (:`then_0`
        (`self.SetColourThenWhite` 0 255))
      (:`then_1`
        (bind _asbp_rover (cast `/Game/UniDidStuff/Player/BP_Rover` (`GameplayStatics.GetPlayerPawn` 0)))
        (`/Game/UniDidStuff/Player/BP_Rover.KickOut` _asbp_rover self)
        (`/Game/UniDidStuff/Door/BP_DoorButton.MoveBrah` (`self.DoorToOpen`))))
    (else
      (`self.SetColourThenWhite` 0 0 255))))

(event `self.ReceiveBeginPlay`
  (bind _output_get (set `self.CorrectCode` (`KismetMathLibrary.RandomIntegerInRange` 1000 9999)))
  (`TextRenderComponent.K2_SetText` (`/Game/UniDidStuff/Puzzles/KeyPad/BP_KeyCode.DisplayedClue` (`self.ConnectedClue`)) (`KismetTextLibrary.Conv_IntToText` _output_get false false)))

(fn `AddNumberToScreen`
  (params (Max :type Integer) (ButtonNumber :type Integer))
  (returns (AddedNumber :type Boolean))
  (locals (AddedNum :type Boolean))
  (bind _screentext (`self.ScreenText`))
  (bind _returnvalue (`KismetTextLibrary.Conv_TextToString` (`TextRenderComponent.Text` _screentext)))
  (bind _output_get (set `local.AddedNum` (< (`KismetStringLibrary.Len` _returnvalue) Max)))
  (if _output_get
    (`TextRenderComponent.K2_SetText` _screentext (`KismetTextLibrary.Conv_StringToText` (`KismetStringLibrary.BuildString_Int` _returnvalue "" ButtonNumber))))
  (return (`local.AddedNum`)))

(fn `BindMyEvents`
  (params (Rover :type "/Game/UniDidStuff/Player/BP_Rover Object Reference"))
  (`parent.BindMyEvents` Rover)
  (`/Game/UniDidStuff/Player/BP_Rover.BindKeyPadPanelStuff` Rover)
  (`/Game/UniDidStuff/Player/BP_Rover.BindKeyPadPanelStuff` Rover)
  (return))

(fn `RemoveLastDigit`
  (bind _screentext (`self.ScreenText`))
  (`TextRenderComponent.K2_SetText` _screentext (`KismetTextLibrary.Conv_StringToText` (`KismetStringLibrary.LeftChop` (`KismetTextLibrary.Conv_TextToString` (`TextRenderComponent.Text` _screentext)) 1))))

(fn `UserConstructionScript`)