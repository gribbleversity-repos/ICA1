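; Puzzle flipper switch that triggers movement on its connected trains when the player clicks its button.
; The trytoflickswitch event runs a short line trace from the mouse cursor and, on a Button hit, calls MoveMyJitty on every connected train.
; A FlipFlop alternates two eased MoveComponentTo rotations to tilt the Rotator back and forth, each stopping the other.
; BindMyEvents extends the parent version by calling BindFlipperPannelStuff with the Rover.
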(event `try to flick switch`
  (bind _rotator (`self.Rotator`))
  (bind (_worldlocation _worlddirection) (`PlayerController.DeprojectMousePositionToWorld` (`GameplayStatics.GetPlayerController` 0)))
  (bind _relativelocation (`SceneComponent.RelativeLocation` _rotator))
  (bind _outhit (`KismetSystemLibrary.LineTraceSingle` :`Start` _worldlocation :`End` (+ _worldlocation (* _worlddirection 500)) :`TraceChannel` "TraceTypeQuery1" :`DrawDebugType` "ForDuration" :`bIgnoreSelf` false :`DrawTime` 0.2))
  (if (== (`.HitComponent` (`GameplayStatics.BreakHitResult` _outhit)) (`self.Button`))
    (for _array_element (`self.ConnectedTrain(s)`)
      (`/Game/UniDidStuff/Train/BP_Train.MoveMyJitty` _array_element))
    (`/Engine/EditorBlueprintResources/StandardMacros.FlipFlop`
      (:`A`
        (`|ExecutionSequence`
          (:`then_0`
            (`KismetSystemLibrary.MoveComponentTo` _rotator _relativelocation (struct :`Pitch` 90.0 :`Roll` 45.0) true true 0.2 true :!label _label))
          (:`then_1`
            (goto _label_2 :!via `Stop`))))
      (:`B`
        (`|ExecutionSequence`
          (:`then_0`
            (`KismetSystemLibrary.MoveComponentTo` _rotator _relativelocation (struct :`Pitch` 90.0 :`Roll` -45.0) true true 0.2 true :!label _label_2))
          (:`then_1`
            (goto _label :!via `Stop`)))))))

(fn `BindMyEvents`
  (params (Rover :type "/Game/UniDidStuff/Player/BP_Rover Object Reference"))
  (`parent.BindMyEvents` Rover)
  (`/Game/UniDidStuff/Player/BP_Rover.BindFlipperPannelStuff` Rover)
  (`/Game/UniDidStuff/Player/BP_Rover.BindFlipperPannelStuff` Rover))

(fn `UserConstructionScript`)