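; BP_WireBox is a wire puzzle box where the player drags cables from left-side nodes onto right-side nodes with the mouse.
; Grabs sphere-trace under the cursor to pick or unplug a cable, and a timeline moves its free end to the line-trace point.
; Releases attach to free right nodes, recording occupancy in component tags, or animate the cable back.
; BindMyEvents has the Rover bind the panel; no solution check exists here.
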(event `AttemptWireGrab`
  (bind (_worldlocation _worlddirection) (`PlayerController.DeprojectMousePositionToWorld` (`GameplayStatics.GetPlayerController` 0)))
  (bind _outhit (`KismetSystemLibrary.SphereTraceSingleForObjects` :`Start` _worldlocation :`End` (+ _worldlocation (* _worlddirection 500)) :`Radius` 5.0 :`ObjectTypes` (`|MakeArray` "ObjectTypeQuery2" :!type "EObjectTypeQuery Enum") :`DrawDebugType` "ForDuration" :`bIgnoreSelf` false :`DrawTime` 0.2))
  (`|ExecutionSequence`
    (:`then_0`
      (goto _label :!via `Open`))
    (:`then_1`
      (for _array_element (`SceneComponent.GetChildrenComponents` (`self.LeftSide`) false)
        (bind (_bblockinghit _binitialoverlap _time _distance _location _impactpoint _normal _impactnormal _physmat _hitactor _hitcomponent) (`GameplayStatics.BreakHitResult` _outhit))
        (if (== _array_element _hitcomponent)
          (`|ExecutionSequence`
            (:`then_0`
              (break))
            (:`then_1`
              (goto _label :!via `Close`))
            (:`then_2`
              (set `self.GrabbedCable` (`KismetStringLibrary.Conv_StringToInt` (`KismetStringLibrary.Conv_NameToString` (`|GetArrayItem` (`ActorComponent.ComponentTags` _hitcomponent)))))
              (`self.GrabWire`)))))
      (`/Engine/EditorBlueprintResources/StandardMacros.Gate` true :!label _label
        (:`Exit`
          (for _array_element_2 (`SceneComponent.GetChildrenComponents` (`self.RightSide`) false)
            (if (== _array_element_2 _hitcomponent)
              (`|ExecutionSequence`
                (:`then_0`
                  (break))
                (:`then_1`
                  (bind _componenttags (`ActorComponent.ComponentTags` _array_element_2))
                  (if (`KismetArrayLibrary.Array_IsValidIndex` _componenttags 1)
                    (set `self.GrabbedCable` (`KismetStringLibrary.Conv_StringToInt` (`KismetStringLibrary.Conv_NameToString` (`|GetArrayItem` _componenttags 1))))
                    (`self.GrabWire`)
                    (else
                      (`KismetSystemLibrary.PrintString` "not today my friend"))))))))))))

(event `GrabWire`
  (for _array_element (`SceneComponent.GetChildrenComponents` (`self.RightSide`) false)
    (bind (_bblockinghit _binitialoverlap _time _distance _location _impactpoint _normal _impactnormal _physmat _hitactor _hitcomponent) (`GameplayStatics.BreakHitResult` (stale `AttemptWireGrab` _outhit)))
    (if (== _hitcomponent _array_element)
      (`|ExecutionSequence`
        (:`then_0`
          (break))
        (:`then_1`
          (`/Engine/EditorBlueprintResources/StandardMacros.IsValid` _hitcomponent
            (:`Is Valid`
              (`KismetArrayLibrary.Array_Remove` (`ActorComponent.ComponentTags` _hitcomponent) 1))
            (:`Is Not Valid`
              _))
          (bind _children (`SceneComponent.GetChildrenComponents` (`self.Cables`) false :!label _label_2))
          (bind _ascable_component (cast `CableComponent` (`|GetArrayItem` _children (`self.GrabbedCable`))))
          (bind _output_get (set `self.CurrentlySelectedCable` _ascable_component))
          (`|ExecutionSequence`
            (:`then_0`
              (set `CableComponent.CableLength` 10.0 _output_get)
              (set `CableComponent.SolverIterations` 5 _output_get)
              (`CableComponent.SetAttachEndToComponent` _output_get (`self.Cables`) "None")
              (`self.AllowReleasing`))
            (:`then_1`
              (`Timeline|UpdateWireEndPoint` :!label _label_3
                (:`Update`
                  (bind __hit_end_pos (`self.MouseScreenLineTrace`))
                  (bind _returnvalue (`KismetMathLibrary.InverseTransformLocation` (`SceneComponent.K2_GetComponentToWorld` (`self.Cables`)) __hit_end_pos))
                  (`KismetSystemLibrary.PrintString` (`KismetStringLibrary.Conv_VectorToString` _returnvalue) true true (struct :`R` 0.85 :`G` 0.681164 :`A` 1.0) 2.0 "h08735pa")
                  (set `CableComponent.EndLocation` _returnvalue (`self.CurrentlySelectedCable`))))))))))
  (for _array_element_2 (`SceneComponent.GetChildrenComponents` (`self.LeftSide`) false)
    (if (== _hitcomponent _array_element_2)
      (`|ExecutionSequence`
        (:`then_0`
          (break))
        (:`then_1`
          (for _array_element_3 (`SceneComponent.GetChildrenComponents` (`self.RightSide`) false)
            (bind _componenttags (`ActorComponent.ComponentTags` _array_element_3))
            (if (== (`|GetArrayItem` _componenttags 1) (`|GetArrayItem` (`ActorComponent.ComponentTags` _array_element_2)))
              (`|ExecutionSequence`
                (:`then_0`
                  (break))
                (:`then_1`
                  (`KismetArrayLibrary.Array_Remove` _componenttags 1)
                  (goto _label_2)))))
          (goto _label_2)))))
  (goto _label_2))

(event `StopUpdatingWireEndPoint`
  (goto _label_3 :!via `Stop`))

(event `ReleaseWire`
  (bind _currentlyselectedcable (`self.CurrentlySelectedCable`))
  (`/Engine/EditorBlueprintResources/StandardMacros.Gate` true :!label _label_4
    (:`Exit`
      (`self.StopUpdatingWireEndPoint`)
      (bind (__hit_end_pos _hitcomponent) (`self.MouseScreenLineTrace`))
      (for _array_element (`SceneComponent.GetChildrenComponents` (`self.RightSide`) false)
        (if (== _array_element _hitcomponent)
          (`|ExecutionSequence`
            (:`then_0`
              (break))
            (:`then_1`
              (`self.LockInWire` _hitcomponent)))))
      (set `self.GrabbedCable` 1000 :!label _label_5)
      (bind _output_get (set `self.LastCashedEndLocation` (`CableComponent.EndLocation` (`self.CurrentlySelectedCable`))))
      (bind (_direction _lerp_alpha _cablelength _solveriterations) (`Timeline|ReturnWireToStartingNode` :!via `PlayFromStart`)
        (:`Update`
          (set `CableComponent.CableLength` _cablelength _currentlyselectedcable)
          (set `CableComponent.SolverIterations` (`KismetMathLibrary.Round` _solveriterations) _currentlyselectedcable)
          (set `CableComponent.EndLocation` (`KismetMathLibrary.VLerp` _output_get (+ (`SceneComponent.RelativeLocation` (`self.CurrentlySelectedCable`)) (-10.0 10.0 0.0)) _lerp_alpha) _currentlyselectedcable))))))

(event `AllowReleasing`
  (goto _label_4 :!via `Open`))

(event `DisallowReleasing`
  (goto _label_4 :!via `Close`))

(event `ReleaseAnyway`
  (goto _label_5))

(event `LockInWire`
  (params (EndNode :type "PrimitiveComponent Object Reference"))
  (if (`KismetArrayLibrary.Array_IsValidIndex` (`ActorComponent.ComponentTags` EndNode) 1)
    (`self.ReleaseAnyway`)
    (`self.DisallowReleasing`)
    (`KismetSystemLibrary.PrintString` "that alr has one in lil jit yeah yeah")
    (elif (`KismetSystemLibrary.IsValid` EndNode)
      (`CableComponent.SetAttachEndToComponent` (`self.CurrentlySelectedCable`) EndNode "None")
      (`KismetArrayLibrary.Array_Set` (`ActorComponent.ComponentTags` EndNode) 1 (`KismetStringLibrary.Conv_StringToName` (`KismetStringLibrary.Conv_IntToString` (`self.GrabbedCable`))) true)
      (`self.DisallowReleasing`))))

(fn `BindMyEvents`
  (params (Rover :type "/Game/UniDidStuff/Player/BP_Rover Object Reference"))
  (`/Game/UniDidStuff/Player/BP_Rover.BindWireBoxPanelStuff` Rover))

(fn `MouseScreenLineTrace`
  (returns (`(Hit/End)Pos` :type "Vector Structure") (HitComponent :type "PrimitiveComponent Object Reference"))
  (bind (_worldlocation _worlddirection) (`PlayerController.DeprojectMousePositionToWorld` (`GameplayStatics.GetPlayerController` 0)))
  (bind _outhit (`KismetSystemLibrary.LineTraceSingle` :`Start` _worldlocation :`End` (+ _worldlocation (* _worlddirection 100)) :`TraceChannel` "TraceTypeQuery1" :`DrawDebugType` "ForOneFrame" :`bIgnoreSelf` false))
  (bind (_bblockinghit _binitialoverlap _time _distance _location _impactpoint _normal _impactnormal _physmat _hitactor _hitcomponent _hitbonename _bonename _hititem _elementindex _faceindex _tracestart _traceend) (`GameplayStatics.BreakHitResult` _outhit))
  (return (`KismetMathLibrary.SelectVector` _impactpoint _traceend _bblockinghit) _hitcomponent))

(fn `UserConstructionScript`)